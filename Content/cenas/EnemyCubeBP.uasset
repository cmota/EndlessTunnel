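; EnemyCubeBP is an enemy cube that launches itself along the reverse of its mesh's forward vector when play begins.
; BeginPlay sets a fixed physics linear velocity on the static mesh, with no per-tick movement logic.
; It also sets the actor's uniform scale once from a cosine of its world X position, so size varies with starting location.
; A debug print of that X value has screen output turned off.
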(event EventBeginPlay
  (bind _returnvalue (Transformation|GetActorLocation))
  (bind _staticmeshcomponent (Variables|Debug|GetStaticMeshComponent))
  (bind _x (Math|Vector|BreakVector _returnvalue))
  (Physics|SetPhysicsLinearVelocity _staticmeshcomponent (* (Math|Vector|GetForwardVector _staticmeshcomponent) -3.5e+03) false "None")
  (Transformation|SetActorScale3D (+ "1.500000,1.500000,1.500000" (Math|Trig|Cos(Radians) (Math|Float|MultiplybyPi (Math|Float|Absolute(Float) (/ _x 5e+03))))))
  (Development|PrintString (Utilities|String|Append (Variables|Default|GetdebugTeste) (Utilities|String|ToString(Float) _x)) false))

(event Collision|EventActorBeginOverlap
  (params (OtherActor :type Actor%20Object%20Reference)))

(event EventTick
  (params (DeltaSeconds :type Float%20%28single-precision%29)))

(fn ConstructionScript)